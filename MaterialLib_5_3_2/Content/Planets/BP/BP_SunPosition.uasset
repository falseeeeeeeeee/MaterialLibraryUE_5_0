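; BP_SunPosition is a placeable marker actor that defines the sun's position and range for planet materials.
; Its construction script toggles the Sphere's visibility via ShowSphere, then writes the actor's location as SunPosition and X scale as SunRange into the MPC_Planet parameter collection.
; Values refresh only when construction reruns; the event graph holds only disabled events and unconnected nodes.
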(event EventBeginPlay)

(event Collision|EventActorBeginOverlap
  (params (OtherActor :type Actor%20Object%20Reference)))

(event EventTick
  (params (DeltaSeconds :type Float%20%28single-precision%29)))

(fn ConstructionScript
  (bind _returnvalue (Transformation|GetActorLocation))
  (Utilities|FlowControl|Sequence
    (:then_0
      (Rendering|SetVisibility (Variables|Default|GetSphere) (Variables|Default|GetbShowSphere) false))
    (:then_1
      (Rendering|Material|SetVectorParameterValue "/Game/Planets/Materials/MPC/MPC_Planet.MPC_Planet" "SunPosition" (Math|Color|MakeColor (.x _returnvalue) (.y _returnvalue) (.z _returnvalue)) :!class /Script/Engine.KismetMaterialLibrary)
      (Rendering|Material|SetScalarParameterValue "/Game/Planets/Materials/MPC/MPC_Planet.MPC_Planet" "SunRange" (.X (Math|Vector|BreakVector (Transformation|GetActorScale3D))) :!class /Script/Engine.KismetMaterialLibrary))))